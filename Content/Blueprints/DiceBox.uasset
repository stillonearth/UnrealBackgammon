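; DiceBox is an actor that rolls two physics-driven Zarik dice when its static mesh is touched and prints the values they land on.
; A touch destroys the old dice, spawns two above the mesh and gives each a random impulse.
; While rolling, Tick checks for all dice reaching zero velocity, then GetHighestFaces reads each value from the index of its highest marker sphere.
; IsRolling is never cleared, so results print every tick while the dice rest.
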(event `self.ReceiveTick`
  (params (DeltaSeconds :type "Float (single-precision)"))
  (bind _stringarray (`self.stringArray`))
  (if (`self.isRolling`)
    (for _array_element (`self.zarikArray`)
      (if (== (`SceneComponent.GetComponentVelocity` (`/Game/Blueprints/zarik.Dice` _array_element)) (0.0 0.0 0.0))
        (set `self.diceHaveStopped` true)
        (else
          (set `self.diceHaveStopped` false)
          (break))))
    (if (`self.diceHaveStopped`)
      (`KismetSystemLibrary.PrintText` "Dice have Stopped")
      (bind _return (`self.GetHighestFaces`))
      (`KismetArrayLibrary.Array_Clear` _stringarray)
      (for _array_element_2 _return
        (`KismetArrayLibrary.Array_Add` _stringarray (`KismetStringLibrary.Conv_IntToString` _array_element_2)))
      (`KismetSystemLibrary.PrintText` (`KismetTextLibrary.Conv_StringToText` (`KismetStringLibrary.JoinStringArray` (`self.stringArray`) ",  "))))))

(event `self.ReceiveBeginPlay`
  (bind _asplayer_character (cast `/Game/Blueprints/PlayerCharacter` (`GameplayStatics.GetPlayerCharacter` 0)))
  (set `self.playerCharacter` _asplayer_character))

(event `self.StaticMesh.OnInputTouchBegin`
  (params (FingerIndex :type "ETouchIndex Enum" :default "Touch1") (TouchedComponent :type "PrimitiveComponent Object Reference"))
  (bind _maximpulse (`self.MaxImpulse`))
  (bind _zarikarray (`self.zarikArray`))
  (bind _zarikarray_2 (`self.zarikArray`))
  (for _array_element _zarikarray
    (`self.K2_DestroyActor` _array_element))
  (`KismetArrayLibrary.Array_Clear` _zarikarray)
  (bind _returnvalue (`|SpawnActorFromClass` "/Game/Blueprints/zarik.zarik_C" (`KismetMathLibrary.MakeTransform` (`KismetMathLibrary.MakeVector` (.x (`SceneComponent.K2_GetComponentLocation` (`self.StaticMesh`))) (.y (`SceneComponent.K2_GetComponentLocation` (`self.StaticMesh`))) (+ (.z (`SceneComponent.K2_GetComponentLocation` (`self.StaticMesh`))) 2000.0)) (struct :`Pitch` 45.0 :`Yaw` 45.0 :`Roll` 45.0)) "Undefined" "OverrideRootScale" null null))
  (`KismetArrayLibrary.Array_Add` _zarikarray_2 _returnvalue)
  (bind _returnvalue_2 (`|SpawnActorFromClass` "/Game/Blueprints/zarik.zarik_C" (`KismetMathLibrary.MakeTransform` (`KismetMathLibrary.MakeVector` (.x (`SceneComponent.K2_GetComponentLocation` (`self.StaticMesh`))) (.y (`SceneComponent.K2_GetComponentLocation` (`self.StaticMesh`))) (+ (.z (`SceneComponent.K2_GetComponentLocation` (`self.StaticMesh`))) 1000.0)) (struct :`Pitch` 45.0 :`Yaw` 45.0 :`Roll` 45.0)) "Undefined" "OverrideRootScale" null null))
  (`KismetArrayLibrary.Array_Add` _zarikarray_2 _returnvalue_2)
  (`KismetSystemLibrary.Delay` 0.0)
  (`PrimitiveComponent.AddImpulse` (`/Game/Blueprints/zarik.Dice` _returnvalue_2) (`KismetMathLibrary.MakeVector` (`KismetMathLibrary.RandomFloatInRange` -10.0 _maximpulse) (`KismetMathLibrary.RandomFloatInRange` -10.0 _maximpulse) (`KismetMathLibrary.RandomFloatInRange` -10.0 _maximpulse)) "None" false)
  (`PrimitiveComponent.AddImpulse` (`/Game/Blueprints/zarik.Dice` _returnvalue) (`KismetMathLibrary.MakeVector` (`KismetMathLibrary.RandomFloatInRange` -10.0 _maximpulse) (`KismetMathLibrary.RandomFloatInRange` -10.0 _maximpulse) (`KismetMathLibrary.RandomFloatInRange` -10.0 _maximpulse)) "None" false)
  (set `self.isRolling` true)
  (set `self.diceHaveStopped` false))

(fn `GetHighestFaces`
  (returns (return :type "Array of Integer"))
  (bind _dices (`self.dices`))
  (`KismetArrayLibrary.Array_Clear` (`self.dices`))
  (for _array_element (`self.zarikArray`)
    (set `self.highestZ` -100.0)
    (bind _output_get (set `self.highestValue` -1))
    (for (_array_element_2 _array_index) (`/Game/Blueprints/zarik.sphereArray` _array_element)
      (bind _z (.z (`SceneComponent.K2_GetComponentLocation` _array_element_2)))
      (if (> _z (`self.highestZ`))
        (set `self.highestZ` _z)
        (set `self.highestValue` (+ _array_index 1))))
    (`KismetArrayLibrary.Array_Add` _dices _output_get))
  (return _dices))

(fn `UserConstructionScript`)