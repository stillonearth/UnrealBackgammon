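; Blueprint actor zarik that collects its six sphere members, Sphere1 through Sphere6, into an array.
; BeginPlay appends the spheres to SphereArray in numeric order.
; The overlap and Tick events are disabled stubs, the construction script is empty, and nothing in these graphs reads the array.
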(event `self.ReceiveBeginPlay`
  (bind _spherearray (`self.sphereArray`))
  (`KismetArrayLibrary.Array_Add` _spherearray (`self.Sphere-1`))
  (`KismetArrayLibrary.Array_Add` _spherearray (`self.Sphere-2`))
  (`KismetArrayLibrary.Array_Add` _spherearray (`self.Sphere-3`))
  (`KismetArrayLibrary.Array_Add` _spherearray (`self.Sphere-4`))
  (`KismetArrayLibrary.Array_Add` _spherearray (`self.Sphere-5`))
  (`KismetArrayLibrary.Array_Add` _spherearray (`self.Sphere-6`)))

(fn `UserConstructionScript`)